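; BP_TowerPawn is a tower pawn that fires on a repeating timer while a tank is in its attack range.
; Overlap begin identifies the tank via GetTankReferenceMessage, stores it in Tank and loops "Fire" by name at ShootDelay.
; Overlap end nulls BPTank and clears the timer, without checking which actor left.
; It also reports turret death through CallTurretDied and exposes a helper that sets projectile spawn pitch.
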(event `self.AttackRange.OnComponentBeginOverlap`
  (params (OverlappedComponent :type "PrimitiveComponent Object Reference") (OtherActor :type "Actor Object Reference") (OtherComp :type "PrimitiveComponent Object Reference") (OtherBodyIndex :type Integer) (bFromSweep :type Boolean) (SweepResult :type "HitResult Structure (by ref)"))
  (bind _bp_tank (message `/Game/Dynamic/Blueprints/Tank/Interfaces/INT_Tank.Get Tank Reference` OtherActor))
  (`/Engine/EditorBlueprintResources/StandardMacros.IsValid` _bp_tank
    (:`Is Valid`
      (set `self.Tank` _bp_tank)
      (bind _returnvalue (`KismetSystemLibrary.K2_SetTimer` null "Fire" (`self.ShootDelay`) true))
      (set `self.Timer` _returnvalue))))

(event `self.AttackRange.OnComponentEndOverlap`
  (params (OverlappedComponent :type "PrimitiveComponent Object Reference") (OtherActor :type "Actor Object Reference") (OtherComp :type "PrimitiveComponent Object Reference") (OtherBodyIndex :type Integer))
  (set `self.BP Tank` null)
  (`KismetSystemLibrary.K2_ClearAndInvalidateTimerHandle` (`self.Timer`)))

(event `self.OnTurretDeath`
  (`self.Turret Died` self))

(fn `Set Projectile Spawn Point Rotation`
  (params (NewRotation_Pitch :type "Float (single-precision)"))
  (bind _projectilespawnpoint (`self.ProjectileSpawnPoint`))
  (bind (_returnvalue_roll _returnvalue_pitch _returnvalue_yaw) (`KismetMathLibrary.BreakRotator` (`SceneComponent.K2_GetComponentRotation` _projectilespawnpoint)))
  (`SceneComponent.K2_SetWorldRotation` _projectilespawnpoint (`KismetMathLibrary.MakeRotator` _returnvalue_roll NewRotation_Pitch _returnvalue_yaw) false false))

(fn `UserConstructionScript`)