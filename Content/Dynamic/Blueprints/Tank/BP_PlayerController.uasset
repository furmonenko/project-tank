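; Player controller for the tank game that owns the local player's UI: start screen, tank HUD and win/lose screen.
; BeginPlay shows the start widget and binds InitController to the game state's game-started event.
; InitController creates the HUD and binds the possessed tank's won, lost and died events to show results or hide the HUD.
; Update events forward ammo and health values to the HUD.
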(event `self.ReceiveBeginPlay`
  (bind _astanks_game_state (cast `TanksGameState` (`GameplayStatics.GetGameState`)))
  (add `TanksGameState.GameStarted` _astanks_game_state (delegate `Init Controller`))
  (if (`self.IsLocalController` self)
    (bind _returnvalue (`|CreateWidget` "/Game/Dynamic/Blueprints/UI/WBP_StartGame.WBP_StartGame_C"))
    (`UserWidget.AddToViewport` _returnvalue 0)))

(event `Init Controller`
  (`self.Create HUD`)
  (bind _astank_pawn (cast `TankPawn` (`self.K2_GetPawn`)))
  (set `self.As Tank Pawn` _astank_pawn)
  (add `TurretPawn.WonGame` (`self.As Tank Pawn`) (delegate `Won Game`))
  (add `TurretPawn.LostGame` (`self.As Tank Pawn`) (delegate `Lost Game`))
  (add `TankPawn.TankDied` (`self.As Tank Pawn`) (delegate `Hide HUD`)))

(event `Hide HUD`
  (bind _hud (`self.HUD`)
    (:`then`
      (set `Widget.Visibility` "Hidden" _hud))
    (:`else`)))

(event `Won Game`
  (bind _returnvalue (`|CreateWidget` "/Game/Dynamic/Blueprints/UI/WBP_Win_Lose.WBP_Win_Lose_C" self))
  (`UserWidget.AddToViewport` _returnvalue 0)
  (`/Game/Dynamic/Blueprints/UI/WBP_Win_Lose.On Game Won` _returnvalue)
  (`self.Hide HUD`))

(event `Lost Game`
  (bind _returnvalue (`|CreateWidget` "/Game/Dynamic/Blueprints/UI/WBP_Win_Lose.WBP_Win_Lose_C" self))
  (`UserWidget.AddToViewport` _returnvalue 0)
  (`/Game/Dynamic/Blueprints/UI/WBP_Win_Lose.On Game Lost` _returnvalue)
  (`self.Hide HUD`))

(event `self.UpdateHUDAmmoCount`
  (params (NewAmmo :type Integer))
  (`/Engine/EditorBlueprintResources/StandardMacros.IsValid` (`self.HUD`)
    (:`Is Valid`
      (`/Game/Dynamic/Blueprints/UI/WBP_Tank_HUD.Set Ammo` (`self.HUD`) NewAmmo))))

(event `self.UpdateHUDHealth`
  (params (NewHealth :type "Float (single-precision)") (MaxHealth :type "Float (single-precision)"))
  (`/Engine/EditorBlueprintResources/StandardMacros.IsValid` (`self.HUD`)
    (:`Is Valid`
      (`/Game/Dynamic/Blueprints/UI/WBP_Tank_HUD.Set Health` (`self.HUD`) NewHealth MaxHealth))))

(fn `Create HUD`
  (if (`self.IsLocalPlayerController`)
    (bind _returnvalue (`|CreateWidget` "/Game/Dynamic/Blueprints/UI/WBP_Tank_HUD.WBP_Tank_HUD_C" self))
    (bind _output_get (set `self.HUD` _returnvalue))
    (`UserWidget.AddToViewport` _output_get 0)))

(fn `Get BP Player Controller`
  (returns (BP_PlayerController :type "/Game/Dynamic/Blueprints/Tank/BP_PlayerController Object Reference"))
  (return self))

(fn `UserConstructionScript`)