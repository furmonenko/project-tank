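; BP_Tank is the player-controllable tank, handling Enhanced Input for movement, turning, looking and firing.
; On BeginPlay it adds its mapping context to the player controller's input subsystem.
; Input events forward to Move, Turn and Fire, whose logic lives outside these graphs, and releasing move zeroes MovementSpeed.
; Look input only passes a zero rotation to SetTargetLookRotation, and GetTankReference returns self.
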(event `self.ReceiveBeginPlay`
  (bind _asplayer_controller (cast `PlayerController` (`self.GetController`)))
  (bind _returnvalue (pcsubsystem `EnhancedInputLocalPlayerSubsystem` _asplayer_controller))
  (`/Engine/EditorBlueprintResources/StandardMacros.IsValid` _returnvalue
    (:`Is Valid`
      (`EnhancedInputSubsystemInterface.AddMappingContext` _returnvalue (`self.Mapping Context`) 0 (struct)))))

(event `EnhancedInput|/Game/Dynamic/Blueprints/Tank/Input/IA_TankMove`
  (params (ActionValue :type "Float (double-precision)") (ElapsedSeconds :type "Float (double-precision)") (TriggeredSeconds :type "Float (double-precision)") (InputAction :type "InputAction Object Reference" :default "/Game/Dynamic/Blueprints/Tank/Input/IA_TankMove.IA_TankMove"))
  (:`Triggered`
    (`self.Move` ActionValue))
  (:`Completed`
    (set `self.MovementSpeed` 0.0)))

(event `EnhancedInput|/Game/Dynamic/Blueprints/Tank/Input/IA_TankFire`
  (params (ActionValue :type Boolean) (ElapsedSeconds :type "Float (double-precision)") (TriggeredSeconds :type "Float (double-precision)") (InputAction :type "InputAction Object Reference" :default "/Game/Dynamic/Blueprints/Tank/Input/IA_TankFire.IA_TankFire"))
  (:`Started`
    (`self.Fire`)))

(event `EnhancedInput|/Game/Dynamic/Blueprints/Tank/Input/IA_TankTurn`
  (params (ActionValue :type "Float (double-precision)") (ElapsedSeconds :type "Float (double-precision)") (TriggeredSeconds :type "Float (double-precision)") (InputAction :type "InputAction Object Reference" :default "/Game/Dynamic/Blueprints/Tank/Input/IA_TankTurn.IA_TankTurn"))
  (:`Triggered`
    (`self.Turn` ActionValue)))

(event `EnhancedInput|/Game/Dynamic/Blueprints/Tank/Input/IA_TankLook`
  (params (ActionValue :type "Vector2D Structure") (ElapsedSeconds :type "Float (double-precision)") (TriggeredSeconds :type "Float (double-precision)") (InputAction :type "InputAction Object Reference" :default "/Game/Dynamic/Blueprints/Tank/Input/IA_TankLook.IA_TankLook"))
  (:`Triggered`
    (`self.SetTargetLookRotation` (struct))))

(fn `Get Tank Reference`
  (returns (BP_Tank :type "/Game/Dynamic/Blueprints/Tank/BP_Tank Object Reference"))
  (return self))

(fn `UserConstructionScript`)