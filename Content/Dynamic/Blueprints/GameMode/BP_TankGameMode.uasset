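; Game mode for a tank-versus-towers game: destroying every tower wins, and the player tank's death loses.
; Tower deaths shrink the tower list and enemy count, while damage and shot events refresh HUD health and ammo.
; Either outcome shows the win/lose widget, fires its game event and reopens the level after a delay.
; Setup for tank, HUD, event bindings and countdown widget is disconnected, leaving BeginPlay and InitGame empty.
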(event `OnGameStarted`)

(event `On Countdown Finished`
  (`KismetSystemLibrary.Delay` 1.0))

(event `self.ReceiveBeginPlay`)

(event `Remove Tower`
  (params (Tower :type "/Game/Dynamic/Blueprints/Towers/BP_TowerPawn Object Reference"))
  (`self.Has Won Game?` Tower
    (:`Yes`
      (bind _returnvalue (`|CreateWidget` "/Game/Dynamic/Blueprints/UI/WBP_Win_Lose.WBP_Win_Lose_C"))
      (`UserWidget.AddToViewport` _returnvalue 0)
      (`self.Game Won`)
      (`self.Restart Level`))))

(event `Init Game`)

(event `Player Lost`
  (params (Tank :type "/Game/Dynamic/Blueprints/Tank/BP_Tank Object Reference"))
  (`self.Lose Game` Tank)
  (`self.Restart Level`))

(event `OnTakeAnyDamage_Event`
  (params (DamagedActor :type "Actor Object Reference") (Damage :type "Float (single-precision)") (DamageType :type "DamageType Object Reference") (InstigatedBy :type "Controller Object Reference") (DamageCauser :type "Actor Object Reference"))
  (`/Engine/EditorBlueprintResources/StandardMacros.IsValid` (`self.HUD`)
    (:`Is Valid`
      (`self.Set Health Bar`))))

(event `OnTankShoot`
  (`/Engine/EditorBlueprintResources/StandardMacros.IsValid` (`self.HUD`)
    (:`Is Valid`
      (`self.Set Ammo Count`))))

(fn `Create HUD`
  (params (Tank :type "/Game/Dynamic/Blueprints/Tank/BP_Tank Object Reference"))
  (returns (HUD :type "/Game/Dynamic/Blueprints/UI/WBP_Tank_HUD Object Reference"))
  (bind _returnvalue (`|CreateWidget` "/Game/Dynamic/Blueprints/UI/WBP_Tank_HUD.WBP_Tank_HUD_C"))
  (`UserWidget.AddToViewport` _returnvalue 0)
  (return _returnvalue))

(fn `Enable Tank`
  (returns (BP_Tank :type "/Game/Dynamic/Blueprints/Tank/BP_Tank Object Reference"))
  (bind _bp_tank (message `/Game/Dynamic/Blueprints/Tank/Interfaces/INT_Tank.Get Tank Reference` (`GameplayStatics.GetPlayerPawn` 0)))
  (`/Engine/EditorBlueprintResources/StandardMacros.IsValid` _bp_tank
    (:`Is Valid`
      (`/Game/Dynamic/Blueprints/Tank/BP_Tank.Disable / Enable Tank` _bp_tank false)
      (return _bp_tank))))

(fn `Get Tank Controller`
  (params (Tank :type "/Game/Dynamic/Blueprints/Tank/BP_Tank Object Reference"))
  (returns (BP_PlayerController :type "/Game/Dynamic/Blueprints/Controllers/PlayerController/BP_PlayerController Object Reference"))
  (bind _bp_playercontroller (message `/Game/Dynamic/Blueprints/Controllers/PlayerController/IBP_PlayerController.Get BP Player Controller` (`Pawn.GetController` Tank)))
  (`/Engine/EditorBlueprintResources/StandardMacros.IsValid` _bp_playercontroller
    (:`Is Valid`
      (return _bp_playercontroller))))

(fn `HUD Init`
  (`self.Set Health Bar`)
  (`self.Set Ammo Count`))

(fn `Lose Game`
  (params (Tank :type "/Game/Dynamic/Blueprints/Tank/BP_Tank Object Reference"))
  (bind _output_get (set `self.Tank` Tank))
  (bind _asplayer_controller (cast `PlayerController` (`Pawn.GetController` (`Actor.Instigator` _output_get))))
  (`/Game/Dynamic/Blueprints/Tank/BP_Tank.Disable / Enable Tank` (`self.Tank`) true)
  (bind _returnvalue (`|CreateWidget` "/Game/Dynamic/Blueprints/UI/WBP_Win_Lose.WBP_Win_Lose_C" _asplayer_controller))
  (`UserWidget.AddToViewport` _returnvalue 0)
  (`self.Game Lost`))

(fn `Set Ammo Count`
  (`/Game/Dynamic/Blueprints/UI/WBP_Tank_HUD.Set Ammo` (`self.HUD`) (`/Game/Dynamic/Blueprints/Tank/BP_Tank.Ammo` (`self.BP Tank`))))

(fn `Set Enemies Count`
  (`/Game/Dynamic/Blueprints/UI/WBP_Tank_HUD.Set Enemies Count` (`self.HUD`) (`KismetArrayLibrary.Array_Length` (`self.Towers`))))

(fn `Set Health Bar`
  (bind _bp_tank (`self.BP Tank`))
  (`/Game/Dynamic/Blueprints/UI/WBP_Tank_HUD.Set Health` (`self.HUD`) (`/Game/Dynamic/Blueprints/Tank/BP_Tank.Get Health` _bp_tank) (`/Game/Dynamic/Blueprints/Tank/BP_Tank.Get Max Health` _bp_tank)))

(fn `UserConstructionScript`)